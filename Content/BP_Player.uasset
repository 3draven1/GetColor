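; BP_Player is a player controller that drives a color test in the HUD's ColorUI widget.
; On BeginPlay it caches BP_HUD, sets Game and UI input focused on ColorUI, shows the cursor and adds an Enhanced Input mapping context.
; IA_Action starts the color test on Triggered and pauses it on Canceled.
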(event `self.ReceiveBeginPlay`
  (bind _asbp_hud (cast `/Game/BP_HUD` (`self.GetHUD`)))
  (bind _output_get (set `self.As BP HUD` _asbp_hud))
  (`WidgetBlueprintLibrary.SetInputMode_GameAndUIEx` self (`/Game/BP_HUD.ColorUI` _output_get))
  (set `self.bShowMouseCursor` true)
  (`EnhancedInputSubsystemInterface.AddMappingContext` (subsystem `EnhancedInputLocalPlayerSubsystem`) "/Game/NewInputMappingContext.NewInputMappingContext" 0 (struct)))

(event `EnhancedInput|/Game/IA_Action`
  (params (ActionValue :type Boolean) (ElapsedSeconds :type "Float (double-precision)") (TriggeredSeconds :type "Float (double-precision)") (InputAction :type "InputAction Object Reference" :default "/Game/IA_Action.IA_Action"))
  (bind _colorui (`/Game/BP_HUD.ColorUI` (`self.As BP HUD`)))
  (:`Triggered`
    (`/Game/ColorWidget.StartColorTest` _colorui 1.0))
  (:`Canceled`
    (`/Game/ColorWidget.PauseColorTest` _colorui)))

(fn `UserConstructionScript`)